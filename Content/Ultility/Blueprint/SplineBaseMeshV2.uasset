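; Spline placement actor that scatters copies of a chosen static mesh along an editable spline.
; The construction script divides the spline length by a spacing variable and adds an InstancedStaticMesh instance at each step, in local space.
; Instances can take a random uniform scale between a minimum and maximum, and keep zero rotation instead of following the spline direction.
; Variable names are in Vietnamese, and the event graph holds no active logic.
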(fn `UserConstructionScript`
  (bind `_loại_mesh_muốn_thêm_staticmesh` (break `/Game/Ultility/DataStructure/PointData` (`self.Loại Mesh muốn thêm`)))
  (bind `_kích_thước_của_đối_tượng` (`self.Kích thước của đối tượng`))
  (bind `_khoảng_cách_giữa_các_đối_tượng` (`self.Khoảng cách giữa các đối tượng`))
  (bind _spline (`self.Spline`))
  (`StaticMeshComponent.SetStaticMesh` (`self.InstancedStaticMesh`) `_loại_mesh_muốn_thêm_staticmesh`)
  (for _index (range (+ (`.ReturnValue` (`KismetMathLibrary.FMod` (`SplineComponent.GetSplineLength` _spline) `_khoảng_cách_giữa_các_đối_tượng`)) 1))
    (if (`self.Có sử dụng kích thước ngẫu nhiên`)
      (set `self.Kích thước của đối tượng` (`KismetMathLibrary.RandomFloatInRange` (`self.Kích thước nhỏ nhất`) (`self.Kích thước lớn nhất`)))
      (else
        (set `self.Kích thước của đối tượng` 1.0)))
    (`InstancedStaticMeshComponent.AddInstance` (`self.InstancedStaticMesh`) (`KismetMathLibrary.MakeTransform` (`SplineComponent.GetLocationAtDistanceAlongSpline` _spline (* _index `_khoảng_cách_giữa_các_đối_tượng`) "Local") (struct) (`KismetMathLibrary.MakeVector` `_kích_thước_của_đối_tượng` `_kích_thước_của_đối_tượng` `_kích_thước_của_đối_tượng`)))))