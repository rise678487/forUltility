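; Editor-placed volume that scatters random instances of a chosen static mesh onto surfaces inside a box.
; The construction script sizes the box and runs a Visibility line trace at random points within it for each requested mesh.
; Each hit adds a world-space instance to an instanced mesh component with random yaw and scale, so misses reduce the count.
; Hit locations and invalid settings are printed for debugging; the event graph is empty.
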(fn `UserConstructionScript`
  (bind (_returnvalue_roll _returnvalue_pitch _returnvalue_yaw) (`KismetMathLibrary.BreakRotator` (`KismetMathLibrary.RandomRotator` false)))
  (bind (_spawnvolumeextent_x _spawnvolumeextent_y _spawnvolumeextent_z) (`KismetMathLibrary.BreakVector` (`self.spawnVolumeExtent`)))
  (bind _meshtospawn (`self.MeshToSpawn`))
  (bind (_spawnvolumeextent_x_2 _spawnvolumeextent_y_2 _spawnvolumeextent_z_2) (`KismetMathLibrary.BreakVector` (`self.spawnVolumeExtent`)))
  (bind _returnvalue (`SceneComponent.K2_GetComponentLocation` (`self.Editor Visual`)))
  (bind _returnvalue_2 (`KismetMathLibrary.RandomFloatInRange` (`self.Min`) (`self.Max`)))
  (bind (_returnvalue_x _returnvalue_y) (`KismetMathLibrary.BreakVector` (`KismetMathLibrary.RandomPointInBoundingBox` _returnvalue (`self.spawnVolumeExtent`))))
  (bind _returnvalue_3 (+ (.z _returnvalue) (/ _spawnvolumeextent_z_2 2.0)))
  (`PrimitiveComponent.SetCastShadow` (`self.SM_Instance`) (`self.bCastShadow`))
  (`BoxComponent.SetBoxExtent` (`self.SpawnVolume`) (`self.spawnVolumeExtent`) true)
  (set `self.lineTraceLength` (* _spawnvolumeextent_z -1.0))
  (if (and (`KismetSystemLibrary.IsValid` _meshtospawn) (> (`self.NumberOfMesh`) 0))
    (`StaticMeshComponent.SetStaticMesh` (`self.SM_Instance`) _meshtospawn)
    (for _ (range (`self.NumberOfMesh`))
      (bind (_outhit _returnvalue_4) (`KismetSystemLibrary.LineTraceSingle` :`Start` (`KismetMathLibrary.MakeVector` _returnvalue_x _returnvalue_y _returnvalue_3) :`End` (`KismetMathLibrary.MakeVector` _returnvalue_x _returnvalue_y (+ _returnvalue_3 (`self.lineTraceLength`))) :`TraceChannel` "TraceTypeQuery1" :`bIgnoreSelf` false))
      (`KismetSystemLibrary.PrintString` (`KismetStringLibrary.Conv_VectorToString` (`.Location` (`GameplayStatics.BreakHitResult` _outhit))))
      (if _returnvalue_4
        (`InstancedStaticMeshComponent.AddInstanceWorldSpace` (`self.SM_Instance`) (`KismetMathLibrary.MakeTransform` (`.Location` (`GameplayStatics.BreakHitResult` _outhit)) (`KismetMathLibrary.MakeRotator` 0.0 0.0 _returnvalue_yaw) (`KismetMathLibrary.MakeVector` _returnvalue_2 _returnvalue_2 _returnvalue_2)))))
    (else
      (`KismetSystemLibrary.PrintString` "Mesh is NULL or number of Mesh is below 0 "))))